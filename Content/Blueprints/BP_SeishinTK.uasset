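; Red Light, Green Light game controller that rotates a Gedo figure and kills players caught moving, starting on the authority after a short delay.
; One timeline, played forward for green and reversed for red, drives the yaw through MulticastRotation.
; When the red turn finishes, every player's velocity is checked once.
; A looping timer then returns to green after a random delay, unless player 0 is safe.
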(event `StartGame`
  (`/Engine/EditorBlueprintResources/ActorMacros.Switch Has Authority`
    (:`Authority`
      (`KismetSystemLibrary.Delay` 3.0)
      (`self.GreenLight`))))

(event `MulticastRotation`
  (params (NewRotation :type "Rotator Structure"))
  (`SceneComponent.K2_SetRelativeRotation` (`self.Gedo`) NewRotation false false))

(event `GreenLight`
  (set `self.CheckForRedOrGreen` false)
  (bind (_direction _newtrack_0) (`Timeline|TurnGedoTimeline` :!via `PlayFromStart` :!label _label)
    (:`Update`
      (`self.MulticastRotation` (`KismetMathLibrary.MakeRotator` 0.0 0.0 _newtrack_0)))
    (:`Finished`
      (if (`self.CheckForRedOrGreen`)
        (bind _returnvalue (`KismetSystemLibrary.K2_SetTimerDelegate` (delegate `CheckForMovement`) 0.1 true true))
        (set `self.CheckPlayerTimer` _returnvalue)
        (for _array_element (`GameStateBase.PlayerArray` (`GameplayStatics.GetGameState`))
          (bind _asbp_first_person_character (cast `/Game/FirstPerson/Blueprints/BP_FirstPersonCharacter` (`PlayerState.GetPawn` _array_element)))
          (if (> (`KismetMathLibrary.VSize` (`self.GetVelocity` _asbp_first_person_character)) 10.0)
            (`/Game/FirstPerson/Blueprints/BP_FirstPersonCharacter.PlayerDeathEvent` _asbp_first_person_character)))
        (else
          (`KismetSystemLibrary.Delay` (`KismetMathLibrary.RandomFloatInRange` 1.0 3.5))
          (`self.RedLight`))))))

(event `RedLight`
  (set `self.CheckForRedOrGreen` true)
  (goto _label :!via `ReverseFromEnd`))

(event `CheckForMovement`
  (bind _asbp_first_person_character (cast `/Game/FirstPerson/Blueprints/BP_FirstPersonCharacter` (`GameplayStatics.GetPlayerCharacter` 0)))
  (if (not (`/Game/FirstPerson/Blueprints/BP_FirstPersonCharacter.IsPlayerSafe?` _asbp_first_person_character))
    (`KismetSystemLibrary.Delay` (`KismetMathLibrary.RandomFloatInRange` 1.0 3.5))
    (`KismetSystemLibrary.K2_ClearAndInvalidateTimerHandle` (`self.CheckPlayerTimer`))
    (`self.GreenLight`)))

(fn `UserConstructionScript`)