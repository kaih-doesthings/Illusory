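; BP_FinishLine is a finish-line trigger that marks players as safe while they are inside its collision volume.
; On server-side begin overlap, a Player-tagged BP_FirstPersonCharacter gets IsPlayerSafe set, and the music audio component on the first BP_StartPlate found in the level is stopped.
; End overlap, also authority-only, clears the safe flag, while the music stays stopped.
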(event `self.CollisionComponent.OnComponentBeginOverlap`
  (params (OverlappedComponent :type "PrimitiveComponent Object Reference") (OtherActor :type "Actor Object Reference") (OtherComp :type "PrimitiveComponent Object Reference") (OtherBodyIndex :type Integer) (bFromSweep :type Boolean) (SweepResult :type "HitResult Structure (by ref)"))
  (`/Engine/EditorBlueprintResources/ActorMacros.Switch Has Authority`
    (:`Authority`
      (if (`self.ActorHasTag` OtherActor "Player")
        (bind _asbp_first_person_character (cast `/Game/FirstPerson/Blueprints/BP_FirstPersonCharacter` OtherActor))
        (bind _outactors (`GameplayStatics.GetAllActorsOfClass` "/Game/Blueprints/BP_StartPlate.BP_StartPlate_C"))
        (`AudioComponent.Stop` (`/Game/Blueprints/BP_StartPlate.MusicAudioComponent` (`|GetArrayItem` _outactors)))
        (set `/Game/FirstPerson/Blueprints/BP_FirstPersonCharacter.IsPlayerSafe?` true _asbp_first_person_character)))))

(event `self.CollisionComponent.OnComponentEndOverlap`
  (params (OverlappedComponent :type "PrimitiveComponent Object Reference") (OtherActor :type "Actor Object Reference") (OtherComp :type "PrimitiveComponent Object Reference") (OtherBodyIndex :type Integer))
  (`/Engine/EditorBlueprintResources/ActorMacros.Switch Has Authority`
    (:`Authority`
      (if (`self.ActorHasTag` OtherActor "Player")
        (bind _asbp_first_person_character (cast `/Game/FirstPerson/Blueprints/BP_FirstPersonCharacter` OtherActor))
        (set `/Game/FirstPerson/Blueprints/BP_FirstPersonCharacter.IsPlayerSafe?` false _asbp_first_person_character)))))

(fn `UserConstructionScript`)